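; RTS-style player controller that creates the HUD, handles box selection and issues orders to selected units.
; Left mouse press and release start and end HUD selection.
; Right-click traces dispatch a unit action or a move, doing nothing when the first trace channel hits.
; Action events write enum and target keys into each selected unit's Blackboard; the resource and resource-building events have no caller in this graph.
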(event Custom|ActionOnResourceBulding
  (params (ResourceBuilding :type BP%20Farm%20Building%20Object%20Reference))
  (for _array_element (Variables|Default|GetSelectedUnits)
    (Utilities|IsValid (AI|GetBlackboard _array_element)
      (:Is%20Valid
        (AI|Components|Blackboard|SetValueasEnum (AI|GetBlackboard _array_element) (Utilities|Name|MakeLiteralName "CollectorActionKey") (Utilities|Enum|LiteralenumE_CollectorAction "NewEnumerator1"))
        (AI|Components|Blackboard|SetValueasObject (AI|GetBlackboard _array_element) (Utilities|Name|MakeLiteralName "TargetResourceBuildingKey") ResourceBuilding)))))

(event Custom|ActionOnResource
  (params (Resource :type BP%20Resources%20Object%20Reference))
  (for _array_element (Variables|Default|GetSelectedUnits)
    (Utilities|IsValid (AI|GetBlackboard _array_element)
      (:Is%20Valid
        (AI|Components|Blackboard|SetValueasEnum (AI|GetBlackboard _array_element) (Utilities|Name|MakeLiteralName "CollectorActionKey") (Utilities|Enum|LiteralenumE_CollectorAction "NewEnumerator0"))
        (AI|Components|Blackboard|SetValueasObject (AI|GetBlackboard _array_element) (Utilities|Name|MakeLiteralName "TargetResourceKey") Resource)))))

(event Custom|ActionOnUnit
  (params (Unit :type BP%20Base%20Unit%20Object%20Reference))
  (for _array_element (Variables|Default|GetSelectedUnits)
    (Utilities|IsValid (AI|GetBlackboard _array_element)
      (:Is%20Valid
        (AI|Components|Blackboard|SetValueasEnum (AI|GetBlackboard _array_element) (Utilities|Name|MakeLiteralName "CombatActionKey") (Utilities|Enum|LiteralenumE_CombatAction "NewEnumerator1"))
        (AI|Components|Blackboard|SetValueasObject (AI|GetBlackboard _array_element) (Utilities|Name|MakeLiteralName "TargetActorKey") Unit)))))

(event EventBeginPlay
  (Input|SetInputModeGameandUI self 0 "LockAlways" false)
  (bind _returnvalue (UserInterface|CreateWidget "/Game/UI/WBP_HUD.WBP_HUD_C"))
  (Variables|Default|SetWidgetHUD _returnvalue)
  (UserInterface|Viewport|AddtoViewport _returnvalue 0))

(event Input|MouseEvents|LeftMouseButton
  (params (Key :type Key%20Structure :default "None"))
  (:Pressed
    (bind _hud (Variables|Default|GetHud)
      (:then
        (Class|RTSHUD|StartSelecting _hud))
      (:else)))
  (:Released
    (bind _hud_2 (Variables|Default|GetHud)
      (:then
        (Class|RTSHUD|EndSelecting _hud_2))
      (:else))))

(event Input|MouseEvents|RightMouseButton
  (params (Key :type Key%20Structure :default "None"))
  (bind (_hitresult _returnvalue) (Game|Player|GetHitResultUnderCursorbyChannel "TraceTypeQuery4" true))
  (:Pressed
    (if (not (.ReturnValue (Game|Player|GetHitResultUnderCursorbyChannel "TraceTypeQuery3" true)))
      (if _returnvalue
        (bind _asbp_base_unit (Utilities|Casting|CastToBP_BaseUnit (.hitactor _hitresult)))
        (CallFunction|ActiononUnit _asbp_base_unit)
        (else
          (Class|RTSPlayerController|MoveSelectedUnits (.location (.HitResult (Game|Player|GetHitResultUnderCursorbyChannel "TraceTypeQuery1" true)))))))))

(fn ConstructionScript)