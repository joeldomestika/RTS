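; Camera pawn that edge-scrolls the view when the mouse nears the borders of the viewport.
; Each Tick runs horizontal and vertical functions that convert the DPI-scaled mouse position into an edge band sized as a percentage of the viewport.
; A clamped normalize helper ramps CameraRoot's relative X and Y movement by depth into that band.
; Movement is a fixed step per frame, not scaled by delta time.
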(event EventBeginPlay)

(event Collision|EventActorBeginOverlap
  (params (OtherActor :type Actor%20Object%20Reference)))

(event EventTick
  (params (DeltaSeconds :type Float%20%28single-precision%29))
  (CallFunction|HorizontalCameraMovement (Variables|Default|GetPercentage))
  (CallFunction|VerticalCameraMovement (Variables|Default|GetPercentage)))

(fn ConstructionScript)

(fn NormalizeValue
  (params (Value :type Float%20%28single-precision%29) (Min :type Float%20%28single-precision%29) (Max :type Float%20%28single-precision%29))
  (return (Math|Float|Clamp(Float) (Math|Float|NormalizetoRange Value Min Max))))

(fn HorizontalCameraMovement
  (params (Percentage :type Float%20%28single-precision%29))
  (Utilities|FlowControl|Sequence
    (:then_0
      (bind _returnvalue (Class|WidgetLayoutLibrary|GetMousePositiononViewport))
      (LocalVariables|SetMouseHorizontalValue (* (.x _returnvalue) (Class|WidgetLayoutLibrary|GetViewportScale))))
    (:then_1
      (LocalVariables|SetCriticalDistance (* (.x (Viewport|GetViewportSize)) (/ Percentage 1e+02))))
    (:then_2
      (Utilities|FlowControl|Sequence
        (:then_0
          (bind _normalizedvalue (CallFunction|NormalizeValue (LocalVariables|GetMouseHorizontalValue) 0.0 (LocalVariables|GetCriticalDistance)))
          (Transformation|AddRelativeLocation (Variables|Default|GetCameraRoot) (* "10.000000, 0, 0" (- 1.0 _normalizedvalue)) false false))
        (:then_1
          (bind _normalizedvalue_2 (CallFunction|NormalizeValue (LocalVariables|GetMouseHorizontalValue) (- (.x (Viewport|GetViewportSize)) (LocalVariables|GetCriticalDistance)) (.x (Viewport|GetViewportSize))))
          (Transformation|AddRelativeLocation (Variables|Default|GetCameraRoot) (* "-10.000000, 0, 0" _normalizedvalue_2) false false))))))

(fn VerticalCameraMovement
  (params (Percentage :type Float%20%28single-precision%29))
  (Utilities|FlowControl|Sequence
    (:then_0
      (bind _returnvalue (Class|WidgetLayoutLibrary|GetMousePositiononViewport))
      (LocalVariables|SetMouseVerticalValue (* (.y _returnvalue) (Class|WidgetLayoutLibrary|GetViewportScale))))
    (:then_1
      (LocalVariables|SetCriticalDistance (* (.y (Viewport|GetViewportSize)) (/ Percentage 1e+02))))
    (:then_2
      (Utilities|FlowControl|Sequence
        (:then_0
          (bind _normalizedvalue (CallFunction|NormalizeValue (LocalVariables|GetMouseVerticalValue) 0.0 (LocalVariables|GetCriticalDistance)))
          (Transformation|AddRelativeLocation (Variables|Default|GetCameraRoot) (* "0.000000,10.000000, 0" (- 1.0 _normalizedvalue)) false false))
        (:then_1
          (bind _normalizedvalue_2 (CallFunction|NormalizeValue (LocalVariables|GetMouseVerticalValue) (- (.y (Viewport|GetViewportSize)) (LocalVariables|GetCriticalDistance)) (.y (Viewport|GetViewportSize))))
          (Transformation|AddRelativeLocation (Variables|Default|GetCameraRoot) (* "0.000000,-10.000000, 0" _normalizedvalue_2) false false))))))