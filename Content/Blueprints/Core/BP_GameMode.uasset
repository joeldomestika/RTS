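; Game mode that holds the wood, food and stone economy for the player and the AI opponent.
; Consume functions deduct only when the balance suffices, returning success and firing that side's resources-changed dispatcher.
; Collect functions fire the dispatcher before adding the amount, so synchronous listeners read the old total.
; The AI alone has a combined cost check and payment, which verifies all three resources before deducting any.
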(event EventBeginPlay)

(event EventTick
  (params (DeltaSeconds :type Float%20%28single-precision%29)))

(fn ConstructionScript)

(fn ConsumeWoodPlayer
  (params (ValueToConsume :type Integer))
  (if (>= (- (Variables|Player|GetWoodCollectedPlayer) ValueToConsume) 0)
    (Variables|Player|SetWoodCollectedPlayer (- (Variables|Player|GetWoodCollectedPlayer) ValueToConsume))
    (Default|CallOnPlayerResourcesChanged)
    (return true)
    (else
      (return false))))

(fn ConsumeFoodPlayer
  (params (ValueToConsume :type Integer))
  (if (>= (- (Variables|Player|GetFoodCollectedPlayer) ValueToConsume) 0)
    (Variables|Player|SetFoodCollectedPlayer (- (Variables|Player|GetFoodCollectedPlayer) ValueToConsume))
    (Default|CallOnPlayerResourcesChanged)
    (return true)
    (else
      (return false))))

(fn ConsumeStonePlayer
  (params (ValueToConsume :type Integer))
  (if (>= (- (Variables|Player|GetStoneCollectedPlayer) ValueToConsume) 0)
    (Variables|Player|SetStoneCollectedPlayer (- (Variables|Player|GetStoneCollectedPlayer) ValueToConsume))
    (Default|CallOnPlayerResourcesChanged)
    (return true)
    (else
      (return false))))

(fn CollectWoodPlayer
  (params (ValueToCollect :type Integer))
  (Default|CallOnPlayerResourcesChanged)
  (Variables|Player|SetWoodCollectedPlayer (+ (Variables|Player|GetWoodCollectedPlayer) ValueToCollect)))

(fn CollectFoodPlayer
  (params (ValueToCollect :type Integer))
  (Default|CallOnPlayerResourcesChanged)
  (Variables|Player|SetFoodCollectedPlayer (+ (Variables|Player|GetFoodCollectedPlayer) ValueToCollect)))

(fn CollectStonePlayer
  (params (ValueToCollect :type Integer))
  (Default|CallOnPlayerResourcesChanged)
  (Variables|Player|SetStoneCollectedPlayer (+ (Variables|Player|GetStoneCollectedPlayer) ValueToCollect)))

(fn ConsumeWoodAI
  (params (ValueToConsume :type Integer))
  (if (>= (- (Variables|AIOpponent|GetWoodCollectedAI) ValueToConsume) 0)
    (Variables|AIOpponent|SetWoodCollectedAI (- (Variables|AIOpponent|GetWoodCollectedAI) ValueToConsume))
    (Default|CallOnAIResourcesChanged)
    (return true)
    (else
      (return false))))

(fn ConsumeFoodAI
  (params (ValueToConsume :type Integer))
  (if (>= (- (Variables|AIOpponent|GetFoodCollectedAI) ValueToConsume) 0)
    (Variables|AIOpponent|SetFoodCollectedAI (- (Variables|AIOpponent|GetFoodCollectedAI) ValueToConsume))
    (Default|CallOnAIResourcesChanged)
    (return true)
    (else
      (return false))))

(fn ConsumeStoneAI
  (params (ValueToConsume :type Integer))
  (if (>= (- (Variables|AIOpponent|GetStoneCollectedAI) ValueToConsume) 0)
    (Variables|AIOpponent|SetStoneCollectedAI (- (Variables|AIOpponent|GetStoneCollectedAI) ValueToConsume))
    (Default|CallOnAIResourcesChanged)
    (return true)
    (else
      (return false))))

(fn CollectWoodAI
  (params (ValueToCollect :type Integer))
  (Default|CallOnAIResourcesChanged)
  (Variables|AIOpponent|SetWoodCollectedAI (+ (Variables|AIOpponent|GetWoodCollectedAI) ValueToCollect)))

(fn CollectFoodAI
  (params (ValueToCollect :type Integer))
  (Default|CallOnAIResourcesChanged)
  (Variables|AIOpponent|SetFoodCollectedAI (+ (Variables|AIOpponent|GetFoodCollectedAI) ValueToCollect)))

(fn CollectStoneAI
  (params (ValueToCollect :type Integer))
  (Default|CallOnAIResourcesChanged)
  (Variables|AIOpponent|SetStoneCollectedAI (+ (Variables|AIOpponent|GetStoneCollectedAI) ValueToCollect)))

(fn CanAIAffordCost
  (params (Wood :type Integer) (Stone :type Integer) (Food :type Integer))
  (return (and (<= Wood (Variables|AIOpponent|GetWoodCollectedAI)) (and (<= Stone (Variables|AIOpponent|GetStoneCollectedAI)) (<= Food (Variables|AIOpponent|GetFoodCollectedAI))))))

(fn AIPaysCost
  (params (Wood :type Integer) (Stone :type Integer) (Food :type Integer))
  (bind _bcanafford (CallFunction|CanAIAffordCost Wood Stone Food))
  (if _bcanafford
    (bind _bsuccess (CallFunction|ConsumeWoodAI Wood))
    (bind _bsuccess_2 (CallFunction|ConsumeStoneAI Stone))
    (bind _bsuccess_3 (CallFunction|ConsumeFoodAI Food))
    (return (and _bsuccess (and _bsuccess_2 _bsuccess_3)))))