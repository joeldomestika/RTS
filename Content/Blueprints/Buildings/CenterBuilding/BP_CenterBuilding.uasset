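; BP_CenterBuilding is a team-owned main building whose destruction ends the match.
; It extends the parent's team responses by swapping the material on three top meshes for player, AI or neutral ownership.
; On BeginPlay it binds to the HealthComponent's death event, which shows WBP_GameFinished, declaring a player win if the building's team is COMPUTER.
; That handler also switches input to UI only and destroys all BP_BaseUnit actors.
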(event Custom|OnBuildingDestroyed
  (params (bIsDead :type Boolean))
  (bind _returnvalue (UserInterface|CreateWidget "/Game/UI/WBP_GameFinished.WBP_GameFinished_C"))
  (bind _output_get (Variables|Default|SetGameFinishedWidget _returnvalue))
  (Default|PlayerHasWon _output_get (Utilities|Enum|Equal(Enum) (Variables|/Script/RTS.HealthComponent|GetTeam (Variables|Default|GetHealthComponent)) "COMPUTER"))
  (UserInterface|Viewport|AddtoViewport (Variables|Default|GetGameFinishedWidget) 0)
  (Input|SetInputModeUIOnly (Game|GetPlayerController 0) (Variables|Default|GetGameFinishedWidget) "LockAlways")
  (bind _outactors (Actor|GetAllActorsOfClass "/Game/Blueprints/Units/BP_BaseUnit.BP_BaseUnit_C"))
  (for _array_element _outactors
    (Utilities|IsValid _array_element
      (:Is%20Valid
        (Actor|DestroyActor _array_element)))))

(event EventBeginPlay
  (|CallParentFunction)
  (EventDispatchers|BindEventtoOnDeath (Variables|Default|GetHealthComponent) (delegate Custom|OnBuildingDestroyed)))

(event Collision|EventActorBeginOverlap
  (params (OtherActor :type Actor%20Object%20Reference))
  (|CallParentFunction OtherActor) ; This node is disabled and will not be called.\nDrag off pins to build functionality.
)

(event EventTick
  (params (DeltaSeconds :type Float%20%28single-precision%29))
  (|CallParentFunction DeltaSeconds) ; This node is disabled and will not be called.\nDrag off pins to build functionality.
)

(event EventOnTeamPlayer
  ;[1 1 1] Respond to Team
  (|CallParentFunction)
  (Rendering|Material|SetMaterial (Variables|Default|GetTopMesh1) 0 "/Game/Blueprints/Buildings/Materials/M_BuildingBasic.M_BuildingBasic"))

(event EventOnTeamNone
  ;[1 1 1] Respond to Team
  (|CallParentFunction)
  (Rendering|Material|SetMaterial (Variables|Default|GetTopMesh1) 0 "/Game/Geometry/Meshes/CubeMaterial.CubeMaterial"))

(event EventOnTeamAI
  ;[1 1 1] Respond to Team
  (|CallParentFunction)
  (Rendering|Material|SetMaterial (Variables|Default|GetTopMesh1) 0 "/Game/Blueprints/Buildings/Materials/M_BuildingBasicAI.M_BuildingBasicAI"))

(fn ConstructionScript
  (|CallParentFunction))