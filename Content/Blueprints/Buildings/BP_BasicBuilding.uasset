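; Base building actor for a team-based strategy game that can be selected by left click, spawns units and can be destroyed.
; Its HealthComponent's team sets gameplay tags and trace-channel blocking at construction, with only player buildings blocking.
; Units spawn at the rally flag inheriting that team, and computer units register with the opponent AI controller.
; Damage routes through HealthComponent, whose events update the health widget and destroy the actor on death.
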(event Custom|SetupHealthBar
  ;[1 1 1] Health Managment
  (bind _aswbp_health (Utilities|Casting|CastToWBP_Health (UserInterface|GetUserWidgetObject (Variables|Default|GetHealthWidgetComponent))))
  (Variables|Default|SetHealthBar _aswbp_health)
  (Variables|/Game/UI/WBP_Health.WBP_Health_C|SetMaxHealth _aswbp_health 1e+02)
  (Variables|/Game/UI/WBP_Health.WBP_Health_C|SetCurrentHealth _aswbp_health 1e+02))

(event Custom|BindHealthEvents
  ;[1 1 1] Health Managment
  ;;[1 1 1] Bind health events
  (EventDispatchers|BindEventtoOnDeath (Variables|Default|GetHealthComponent) (delegate Custom|DeathEvent))
  (EventDispatchers|BindEventtoOnHealthChanged (Variables|Default|GetHealthComponent) (delegate Custom|UpdateHealth)))

(event Custom|UpdateHealth
  (params (NewHealth :type Float%20%28single-precision%29))
  ;[1 1 1] Health Managment
  ;;[1 1 1] Bind health events
  (bind _healthbar (Variables|Default|GetHealthBar)
    (:then
      (Default|UpdateHealth _healthbar NewHealth))
    (:else)))

(event Custom|DeathEvent
  (params (bIsDead :type Boolean))
  ;[1 1 1] Health Managment
  ;;[1 1 1] Bind health events
  (Utilities|FlowControl|Delay 0.2)
  (Actor|DestroyActor))

(event Custom|OnTeamPlayer
  ;[1 1 1] Respond to Team
  (CallFunction|CleanTags)
  (GameplayTags|AddGameplayTag (Variables|Default|GetGameplayTags) "(TagName=\"Team.Player\")" :!class /Script/GameplayTags.BlueprintGameplayTagLibrary)
  (Collision|SetCollisionResponsetoChannel (Variables|Default|GetBuildingMesh) "ECC_GameTraceChannel1" "ECR_Block"))

(event Custom|OnTeamAI
  ;[1 1 1] Respond to Team
  (CallFunction|CleanTags)
  (GameplayTags|AddGameplayTag (Variables|Default|GetGameplayTags) "(TagName=\"Team.AI\")" :!class /Script/GameplayTags.BlueprintGameplayTagLibrary)
  (Collision|SetCollisionResponsetoChannel (Variables|Default|GetBuildingMesh) "ECC_GameTraceChannel1" "ECR_Ignore"))

(event Custom|OnTeamNone
  ;[1 1 1] Respond to Team
  (CallFunction|CleanTags)
  (GameplayTags|AddGameplayTag (Variables|Default|GetGameplayTags) "(TagName=\"Team.None\")" :!class /Script/GameplayTags.BlueprintGameplayTagLibrary)
  (Collision|SetCollisionResponsetoChannel (Variables|Default|GetBuildingMesh) "ECC_GameTraceChannel1" "ECR_Ignore"))

(event Custom|CleanTags
  (GameplayTags|RemoveGameplayTag (Variables|Default|GetGameplayTags) "(TagName=\"Team.AI\")" :!class /Script/GameplayTags.BlueprintGameplayTagLibrary)
  (GameplayTags|RemoveGameplayTag (Variables|Default|GetGameplayTags) "(TagName=\"Team.None\")" :!class /Script/GameplayTags.BlueprintGameplayTagLibrary)
  (GameplayTags|RemoveGameplayTag (Variables|Default|GetGameplayTags) "(TagName=\"Team.Player\")" :!class /Script/GameplayTags.BlueprintGameplayTagLibrary))

(event Custom|BuildUnit
  (params (UnitClass :type RTS%20Unit%20Class%20Reference))
  (bind _returnvalue (Game|SpawnActorfromClass UnitClass (Transformation|GetWorldTransform (Variables|Default|GetRallyFlag)) "AdjustIfPossibleButAlwaysSpawn" 0 0))
  (Variables|/Script/RTS.HealthComponent|SetTeam (Variables|/Script/RTS.RTS_Unit|GetHealthComponent _returnvalue) (Variables|/Script/RTS.HealthComponent|GetTeam (Variables|Default|GetHealthComponent)))
  (bind _asbp_base_unit (Utilities|Casting|CastToBP_BaseUnit _returnvalue))
  (Default|UpdateUnit _asbp_base_unit)
  (switch Utilities|FlowControl|Switch|SwitchonETeam (Variables|/Script/RTS.HealthComponent|GetTeam (Variables|/Script/RTS.RTS_Unit|GetHealthComponent _asbp_base_unit))
    (:COMPUTER
      (bind _aicontrolleropponent (Variables|Default|GetAIControllerOpponent)
        (:then
          (Default|AddUnit _aicontrolleropponent _asbp_base_unit))
        (:else)))))

(event Custom|UpdateBuilding
  (bind _healthcomponent (Variables|Default|GetHealthComponent)
    (:then
      (switch Utilities|FlowControl|Switch|SwitchonETeam (Variables|/Script/RTS.HealthComponent|GetTeam _healthcomponent)
        (:PLAYER
          (CallFunction|OnTeamPlayer))
        (:COMPUTER
          (CallFunction|OnTeamAI))
        (:NONE
          (CallFunction|OnTeamNone))))
    (:else)))

(event EventBeginPlay
  (CallFunction|SetupHealthBar)
  (CallFunction|BindHealthEvents)
  (bind _outactors (Actor|GetAllActorsOfClass "/Game/Blueprints/AI_Opponent/BP_Opponent.BP_Opponent_C"))
  (if (> (Utilities|Array|Length _outactors) 0)
    (bind _asbp_aicontroller_opponent (Utilities|Casting|CastToBP_AIControllerOpponent (AI|GetAIController (Utilities|Array|Get(acopy) _outactors))))
    (Variables|Default|SetAIControllerOpponent _asbp_aicontroller_opponent)))

(event Collision|EventActorBeginOverlap
  (params (OtherActor :type Actor%20Object%20Reference)))

(event EventTick
  (params (DeltaSeconds :type Float%20%28single-precision%29)))

(event Game|Damage|EventAnyDamage
  (params (Damage :type Float%20%28single-precision%29) (DamageType :type Damage%20Type%20Object%20Reference) (InstigatedBy :type Controller%20Object%20Reference) (DamageCauser :type Actor%20Object%20Reference))
  (bind _returnvalue (Transformation|GetActorLocation))
  ;[1 1 1] Health Managment
  (bind _combattype (Class|BPIProjectileInterface|GetCombatType(Message) DamageCauser))
  (bind _team (Class|BPIProjectileInterface|GetCombatTeam(Message) DamageCauser))
  (Class|HealthComponent|AddDamage (Variables|Default|GetHealthComponent) Damage _combattype _team)
  (Class|AISenseDamage|ReportDamageEvent self (Variables|/Script/Engine.Actor|GetInstigator DamageCauser) Damage _returnvalue _returnvalue "None"))

(event MouseInput|EventActorOnClicked
  (params (ButtonPressed :type Key%20Structure :default "None"))
  (if (== ButtonPressed "LeftMouseButton")
    (bind _asbp_player_controller (Utilities|Casting|CastToBP_PlayerController (Game|GetPlayerController 0)))
    (bind _returnvalue (Class|RTSBuilding|GetIsSelected))
    (if _returnvalue
      (Class|RTSPlayerController|UnselectBuilding _asbp_player_controller)
      (else
        (Class|RTSPlayerController|SelectBuilding _asbp_player_controller self)))))

(fn ConstructionScript
  (CallFunction|UpdateBuilding))