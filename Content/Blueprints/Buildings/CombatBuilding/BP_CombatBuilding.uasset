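; BP_CombatBuilding is a building that produces combat units: tanks, assault vehicles and soldiers.
; Each build event passes its unit class to BuildUnit.
; SetupUI casts the building widget to WBP_CombatBuilding and hands it a reference to this building.
; Team events for player, AI and none call the parent, then swap the top mesh material to match ownership.
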(event Custom|BuildTank
  (CallFunction|BuildUnit "/Game/Blueprints/Units/Combat/Tank/BP_Tank.BP_Tank_C"))

(event Custom|BuildAssaultVehicle
  (CallFunction|BuildUnit "/Game/Blueprints/Units/Combat/AssaultVehicle/BP_AssaultVehicle.BP_AssaultVehicle_C"))

(event Custom|BuildSoldier
  (CallFunction|BuildUnit "/Game/Blueprints/Units/Combat/Soldier/BP_Soldier.BP_Soldier_C"))

(event EventBeginPlay
  (|CallParentFunction))

(event Collision|EventActorBeginOverlap
  (params (OtherActor :type Actor%20Object%20Reference))
  (|CallParentFunction OtherActor) ; This node is disabled and will not be called.\nDrag off pins to build functionality.
)

(event EventTick
  (params (DeltaSeconds :type Float%20%28single-precision%29))
  (|CallParentFunction DeltaSeconds) ; This node is disabled and will not be called.\nDrag off pins to build functionality.
)

(event EventOnTeamPlayer
  ;[1 1 1] Respond to Team
  (|CallParentFunction)
  (Rendering|Material|SetMaterial (Variables|Default|GetTopMesh) 0 "/Game/Blueprints/Buildings/Materials/M_BuildingBasic.M_BuildingBasic"))

(event EventOnTeamNone
  ;[1 1 1] Respond to Team
  (|CallParentFunction)
  (Rendering|Material|SetMaterial (Variables|Default|GetTopMesh) 0 "/Game/Geometry/Meshes/CubeMaterial.CubeMaterial"))

(event EventOnTeamAI
  ;[1 1 1] Respond to Team
  (|CallParentFunction)
  (Rendering|Material|SetMaterial (Variables|Default|GetTopMesh) 0 "/Game/Blueprints/Buildings/Materials/M_BuildingBasicAI.M_BuildingBasicAI"))

(event EventSetupUI
  (bind _aswbp_combat_building (Utilities|Casting|CastToWBP_CombatBuilding (Variables|Default|GetBuildingWidget)))
  (Variables|/Game/Blueprints/Buildings/CombatBuilding/UI/WBP_CombatBuilding.WBP_CombatBuilding_C|SetCombatBuilding _aswbp_combat_building self))

(fn ConstructionScript
  (|CallParentFunction))