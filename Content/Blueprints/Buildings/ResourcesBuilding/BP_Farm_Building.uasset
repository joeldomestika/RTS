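; BP_Farm_Building is a farm resource building that can be selected and can build collector units.
; Team events extend the parent's behavior by swapping the extra mesh's material for player, AI or neutral ownership.
; Left click toggles selection through BP_PlayerController, while right click passes the building to the controller's resource-building action.
; SetupUI hands the building to its resource widget, and BuildCollector queues BP_Collector through BuildUnit.
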(event Custom|BuildCollector
  (CallFunction|BuildUnit "/Game/Blueprints/Units/Collectors/BP_Collector.BP_Collector_C"))

(event EventBeginPlay
  (|CallParentFunction) ; This node is disabled and will not be called.\nDrag off pins to build functionality.
)

(event Collision|EventActorBeginOverlap
  (params (OtherActor :type Actor%20Object%20Reference))
  (|CallParentFunction OtherActor) ; This node is disabled and will not be called.\nDrag off pins to build functionality.
)

(event EventTick
  (params (DeltaSeconds :type Float%20%28single-precision%29))
  (|CallParentFunction DeltaSeconds) ; This node is disabled and will not be called.\nDrag off pins to build functionality.
)

(event EventSetupUI
  (bind _aswbp_resource_building (Utilities|Casting|CastToWBP_ResourceBuilding (Variables|Default|GetBuildingWidget)))
  (Variables|/Game/Blueprints/Buildings/ResourcesBuilding/UI/WBP_ResourceBuilding.WBP_ResourceBuilding_C|SetResourcesBuilding _aswbp_resource_building self))

(event EventOnTeamPlayer
  ;[1 1 1] Respond to Team
  (|CallParentFunction)
  (Rendering|Material|SetMaterial (Variables|Default|GetExtraMesh) 0 "/Game/Blueprints/Buildings/Materials/M_BuildingBasic.M_BuildingBasic"))

(event EventOnTeamNone
  ;[1 1 1] Respond to Team
  (|CallParentFunction)
  (Rendering|Material|SetMaterial (Variables|Default|GetExtraMesh) 0 "/Game/Geometry/Meshes/CubeMaterial.CubeMaterial"))

(event EventOnTeamAI
  ;[1 1 1] Respond to Team
  (|CallParentFunction)
  (Rendering|Material|SetMaterial (Variables|Default|GetExtraMesh) 0 "/Game/Blueprints/Buildings/Materials/M_BuildingBasicAI.M_BuildingBasicAI"))

(event MouseInput|EventActorOnClicked
  (params (ButtonPressed :type Key%20Structure :default "None"))
  (if (== ButtonPressed "LeftMouseButton")
    (bind _asbp_player_controller (Utilities|Casting|CastToBP_PlayerController (Game|GetPlayerController 0)))
    (bind _returnvalue (Class|RTSBuilding|GetIsSelected))
    (if _returnvalue
      (Class|RTSPlayerController|UnselectBuilding _asbp_player_controller)
      (else
        (Class|RTSPlayerController|SelectBuilding _asbp_player_controller self)))
    (elif (== ButtonPressed "RightMouseButton")
      (bind _asbp_player_controller_2 (Utilities|Casting|CastToBP_PlayerController (Game|GetPlayerController 0)))
      (Default|ActiononResourceBulding _asbp_player_controller_2 self))))

(fn ConstructionScript
  (|CallParentFunction))