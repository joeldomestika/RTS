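; Construction-site building that stands in while a structure is built, then replaces itself with the finished building.
; BuildBuilding waits a fixed three seconds, spawns the requested class at its root transform, copies the team via HealthComponent, then destroys itself.
; Meanwhile, a looping timer feeds elapsed time to a progress-bar widget.
; Team events override the parent to swap the mesh material for player, AI or no team.
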(event Custom|BuildBuilding
  (params (BuildingClass :type BP%20Basic%20Building%20Class%20Reference))
  (CallFunction|StartTimer)
  (Utilities|FlowControl|Delay 3.0)
  (bind _returnvalue (Game|SpawnActorfromClass BuildingClass (Transformation|GetWorldTransform (Variables|Default|GetBuildingRootComponent)) "AlwaysSpawn" 0 0))
  (bind _healthcomponent (Variables|Default|GetHealthComponent _returnvalue)
    (:then
      (Variables|/Script/RTS.HealthComponent|SetTeam _healthcomponent (Variables|/Script/RTS.HealthComponent|GetTeam (Variables|Default|GetHealthComponent)))
      (Default|UpdateBuilding _returnvalue)
      (Utilities|Time|ClearandInvalidateTimerbyHandle (Variables|Default|GetBuildingTimer))
      (Actor|DestroyActor))
    (:else)))

(event Custom|Setup%20Progress%20Widget
  (bind _aswbp_progress_building (Utilities|Casting|CastToWBP_ProgressBuilding (UserInterface|GetUserWidgetObject (Variables|Default|GetBuildingProgressBarWidget))))
  (Variables|Default|SetAs%20WBP%20Progress%20Building _aswbp_progress_building))

(event Custom|StartTimer
  (bind _as_wbp_progress_building (Variables|Default|GetAs%20WBP%20Progress%20Building)
    (:then
      (Variables|/Game/UI/WBP_ProgressBuilding.WBP_ProgressBuilding_C|SetMaxProgressTime _as_wbp_progress_building 3.0)
      (Variables|/Game/UI/WBP_ProgressBuilding.WBP_ProgressBuilding_C|SetCurrentProgressTime _as_wbp_progress_building 0.0)
      (Rendering|SetVisibility (Variables|Default|GetBuildingProgressBarWidget) true true)
      (bind _returnvalue (Utilities|Time|SetTimerbyEvent (delegate Custom|UpdateTimer) 0.2 true))
      (Variables|Default|SetBuildingTimer _returnvalue))
    (:else)))

(event Custom|UpdateTimer
  (Variables|Default|SetCounter (+ (Variables|Default|GetCounter) 0.2))
  (bind _as_wbp_progress_building (Variables|Default|GetAs%20WBP%20Progress%20Building)
    (:then
      (Default|UpdateProgressTime _as_wbp_progress_building (Variables|Default|GetCounter)))
    (:else)))

(event EventBeginPlay
  (|CallParentFunction)
  (CallFunction|SetupProgressWidget))

(event Collision|EventActorBeginOverlap
  (params (OtherActor :type Actor%20Object%20Reference))
  (|CallParentFunction OtherActor) ; This node is disabled and will not be called.\nDrag off pins to build functionality.
)

(event EventTick
  (params (DeltaSeconds :type Float%20%28single-precision%29))
  (|CallParentFunction DeltaSeconds) ; This node is disabled and will not be called.\nDrag off pins to build functionality.
)

(event EventOnTeamPlayer
  ;[1 1 1] Respond to Team
  (|CallParentFunction)
  (Rendering|Material|SetMaterial (Variables|Default|GetBuildingMesh) 0 "/Game/Blueprints/Buildings/Materials/M_BuildingBasic.M_BuildingBasic"))

(event EventOnTeamNone
  ;[1 1 1] Respond to Team
  (|CallParentFunction)
  (Rendering|Material|SetMaterial (Variables|Default|GetBuildingMesh) 0 "/Game/Geometry/Meshes/CubeMaterial.CubeMaterial"))

(event EventOnTeamAI
  ;[1 1 1] Respond to Team
  (|CallParentFunction)
  (Rendering|Material|SetMaterial (Variables|Default|GetBuildingMesh) 0 "/Game/Blueprints/Buildings/Materials/M_BuildingBasicAI.M_BuildingBasicAI"))

(fn ConstructionScript
  (|CallParentFunction))