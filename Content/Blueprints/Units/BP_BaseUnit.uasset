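; Base unit Blueprint that can be selected, moved and damaged, with a health bar display.
; Left-click toggles selection through BP_PlayerController, right-click passes the unit to its ActionOnUnit, and MoveUnit uses SimpleMoveToLocation on the instigator controller.
; AnyDamage feeds HealthComponent with a fixed opponent type and team.
; The component's bound events update the WBP_Health widget and destroy the actor shortly after death.
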(event Custom|SetupHealthBar
  (bind _aswbp_health (Utilities|Casting|CastToWBP_Health (UserInterface|GetUserWidgetObject (Variables|Default|GetHealthWidgetComponent))))
  (Variables|Default|SetHealthBar _aswbp_health)
  (Variables|/Game/UI/WBP_Health.WBP_Health_C|SetMaxHealth _aswbp_health 1e+02)
  (Variables|/Game/UI/WBP_Health.WBP_Health_C|SetCurrentHealth _aswbp_health 1e+02))

(event Custom|BindHealthEvents
  (EventDispatchers|BindEventtoOnDeath (Variables|Default|GetHealthComponent) (delegate Custom|DeathEvent))
  (EventDispatchers|BindEventtoOnHealthChanged (Variables|Default|GetHealthComponent) (delegate Custom|UpdateHealth)))

(event Custom|UpdateHealth
  (params (NewHealth :type Float%20%28single-precision%29))
  (bind _healthbar (Variables|Default|GetHealthBar)
    (:then
      (Default|UpdateHealth _healthbar NewHealth))
    (:else)))

(event Custom|DeathEvent
  (params (bIsDead :type Boolean))
  (Utilities|FlowControl|Delay 0.2)
  (Actor|DestroyActor))

(event EventBeginPlay
  (CallFunction|SetupHealthBar)
  (CallFunction|BindHealthEvents))

(event Collision|EventActorBeginOverlap
  (params (OtherActor :type Actor%20Object%20Reference)))

(event EventTick
  (params (DeltaSeconds :type Float%20%28single-precision%29)))

(event Game|Damage|EventAnyDamage
  (params (Damage :type Float%20%28single-precision%29) (DamageType :type Damage%20Type%20Object%20Reference) (InstigatedBy :type Controller%20Object%20Reference) (DamageCauser :type Actor%20Object%20Reference))
  (Class|HealthComponent|AddDamage (Variables|Default|GetHealthComponent) Damage "NONE" "COMPUTER"))

(event EventMoveUnit
  (params (Location :type Vector :default "0, 0, 0"))
  (AI|Navigation|SimpleMovetoLocation (Game|GetInstigatorController) Location))

(event MouseInput|EventActorOnClicked
  (params (ButtonPressed :type Key%20Structure :default "None"))
  (if (== ButtonPressed "LeftMouseButton")
    (bind _asbp_player_controller (Utilities|Casting|CastToBP_PlayerController (Game|GetPlayerController 0)))
    (bind _returnvalue (Class|RTSUnit|GetIsSelected))
    (if _returnvalue
      (Class|RTSPlayerController|RemoveSelectedUnit _asbp_player_controller self)
      (else
        (Class|RTSPlayerController|AddSelectedUnit _asbp_player_controller self)))
    (elif (== ButtonPressed "RightMouseButton")
      (bind _asbp_player_controller_2 (Utilities|Casting|CastToBP_PlayerController (Game|GetPlayerController 0)))
      (Default|ActiononUnit _asbp_player_controller_2 self))))

(fn ConstructionScript)