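; AI controller for combat units that picks hostile targets from perception updates.
; On each perception update it refreshes the controlled unit's team, then flags perceived RTS units or buildings whose health component reports a different team.
; Each detection writes the actor to the blackboard target key and sets the combat action enum, so the last hostile processed becomes the target.
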(event OnPerceptionUpdated(AIPerception)
  (params (UpdatedActors :type Array%20of%20Actor%20Object%20References))
  (CallFunction|UpdateTeam)
  (for _array_element UpdatedActors
    (bind _asrts_unit (Utilities|Casting|CastToRTS_Unit _array_element)
      (:then
        (if (Utilities|Enum|NotEqual(Enum) (Variables|/Script/RTS.HealthComponent|GetTeam (Variables|/Script/RTS.RTS_Unit|GetHealthComponent _asrts_unit)) (Variables|Default|GetControlledPawnTeam))
          (CallFunction|ActorDetected _asrts_unit)))
      (:CastFailed
        (bind _asrts_building (Utilities|Casting|CastToRTS_Building _array_element))
        (if (Utilities|Enum|NotEqual(Enum) (Variables|/Script/RTS.HealthComponent|GetTeam (Variables|/Script/RTS.RTS_Building|GetHealthComponent _asrts_building)) (Variables|Default|GetControlledPawnTeam))
          (CallFunction|ActorDetected _asrts_building))))))

(event Custom|UpdateTeam
  (bind _asrts_unit (Utilities|Casting|CastToRTS_Unit (Pawn|GetControlledPawn)))
  (Variables|Default|SetControlledPawnTeam (Variables|/Script/RTS.HealthComponent|GetTeam (Variables|/Script/RTS.RTS_Unit|GetHealthComponent _asrts_unit))))

(event Custom|ActorDetected
  (params (Actor :type Actor%20Object%20Reference))
  (AI|Components|Blackboard|SetValueasObject (AI|GetBlackboard 0) (Utilities|Name|MakeLiteralName "TargetActorKey") Actor)
  (AI|Components|Blackboard|SetValueasEnum (AI|GetBlackboard 0) (Utilities|Name|MakeLiteralName "CombatActionKey") (Utilities|Enum|LiteralenumE_CombatAction "NewEnumerator1")))

(event EventBeginPlay
  (|CallParentFunction) ; This node is disabled and will not be called.\nDrag off pins to build functionality.
)

(event EventTick
  (params (DeltaSeconds :type Float%20%28single-precision%29))
  (|CallParentFunction DeltaSeconds) ; This node is disabled and will not be called.\nDrag off pins to build functionality.
)

(fn ConstructionScript
  (|CallParentFunction))