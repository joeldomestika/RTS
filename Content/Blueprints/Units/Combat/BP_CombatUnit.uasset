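; BP_CombatUnit is a combat unit Blueprint that receives move orders through its blackboard.
; MoveUnit writes the destination to TargetLocationKey and sets CombatActionKey to an E_CombatAction value, leaving the movement itself to logic outside this graph.
; MoveBaby is an empty event, the default event nodes are disabled, and the construction script only calls its parent.
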(event Custom|MoveBaby)

(event EventBeginPlay
  (|CallParentFunction) ; This node is disabled and will not be called.\nDrag off pins to build functionality.
)

(event Collision|EventActorBeginOverlap
  (params (OtherActor :type Actor%20Object%20Reference))
  (|CallParentFunction OtherActor) ; This node is disabled and will not be called.\nDrag off pins to build functionality.
)

(event EventTick
  (params (DeltaSeconds :type Float%20%28single-precision%29))
  (|CallParentFunction DeltaSeconds) ; This node is disabled and will not be called.\nDrag off pins to build functionality.
)

(event EventMoveUnit
  (params (Location :type Vector :default "0, 0, 0"))
  (AI|Components|Blackboard|SetValueasVector (AI|GetBlackboard 0) (Utilities|Name|MakeLiteralName "TargetLocationKey") Location)
  (AI|Components|Blackboard|SetValueasEnum (AI|GetBlackboard 0) (Utilities|Name|MakeLiteralName "CombatActionKey") (Utilities|Enum|LiteralenumE_CombatAction "NewEnumerator0")))

(fn ConstructionScript
  (|CallParentFunction))