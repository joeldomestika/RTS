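; Base projectile actor for unit combat that damages units it touches.
; When its Sphere overlaps a BP_BaseUnit, it applies a fixed amount of damage with itself as causer, then destroys itself; other actors are ignored.
; It stores team and combat type through setters and getters, but the overlap logic checks neither, and GetProjectileCombatType returns NONE rather than the stored type.
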(event OnComponentBeginOverlap(Sphere)
  (params (OverlappedComponent :type Primitive%20Component%20Object%20Reference) (OtherActor :type Actor%20Object%20Reference) (OtherComp :type Primitive%20Component%20Object%20Reference) (OtherBodyIndex :type Integer) (bFromSweep :type Boolean) (SweepResult :type Hit%20Result%20Structure%20%28by%20ref%29))
  (bind _asbp_base_unit (Utilities|Casting|CastToBP_BaseUnit OtherActor))
  (Game|Damage|ApplyDamage _asbp_base_unit 1e+01 0 self)
  (Actor|DestroyActor))

(event EventBeginPlay)

(event Collision|EventActorBeginOverlap
  (params (OtherActor :type Actor%20Object%20Reference)))

(event EventTick
  (params (DeltaSeconds :type Float%20%28single-precision%29)))

(event EventSetCombatTeam
  (params (Team :type ETeam%20Enum :default "PLAYER"))
  (Variables|Default|SetProjectileTeam Team))

(event EventSetCombatType
  (params (CombatType :type ECombatType%20Enum :default "NONE"))
  (Variables|Default|SetProjectileCombatType CombatType))

(fn ConstructionScript)

(fn GetProjectileCombatType
  (return "NONE"))

(fn GetCombatTeam
  (return (Variables|Default|GetProjectileTeam)))

(fn GetCombatType
  (return (Variables|Default|GetProjectileCombatType)))