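; BP_Tank is a tank combat unit whose body reflects the team it belongs to: player, AI or none.
; Each team event calls the parent, then sets the TankBody material and its block or ignore responses on two custom trace channels.
; Player units block GameTraceChannel1 and ignore GameTraceChannel2, while AI and unassigned units do the reverse.
; BeginPlay, overlap and Tick are disabled stubs, and construction only calls the parent.
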(event EventBeginPlay
  (|CallParentFunction) ; This node is disabled and will not be called.\nDrag off pins to build functionality.
)

(event Collision|EventActorBeginOverlap
  (params (OtherActor :type Actor%20Object%20Reference))
  (|CallParentFunction OtherActor) ; This node is disabled and will not be called.\nDrag off pins to build functionality.
)

(event EventTick
  (params (DeltaSeconds :type Float%20%28single-precision%29))
  (|CallParentFunction DeltaSeconds) ; This node is disabled and will not be called.\nDrag off pins to build functionality.
)

(event EventOnTeamPlayerUnit
  (|CallParentFunction)
  (Collision|SetCollisionResponsetoChannel (Variables|Default|GetTankBody) "ECC_GameTraceChannel1" "ECR_Block")
  (Rendering|Material|SetMaterial (Variables|Default|GetTankBody) 0 "/Game/Blueprints/Buildings/Materials/M_BuildingBasic.M_BuildingBasic")
  (Collision|SetCollisionResponsetoChannel (Variables|Default|GetTankBody) "ECC_GameTraceChannel2" "ECR_Ignore"))

(event EventOnTeamAIUnit
  (|CallParentFunction)
  (Collision|SetCollisionResponsetoChannel (Variables|Default|GetTankBody) "ECC_GameTraceChannel1" "ECR_Ignore")
  (Rendering|Material|SetMaterial (Variables|Default|GetTankBody) 0 "/Game/Blueprints/Buildings/Materials/M_BuildingBasicAI.M_BuildingBasicAI")
  (Collision|SetCollisionResponsetoChannel (Variables|Default|GetTankBody) "ECC_GameTraceChannel2" "ECR_Block"))

(event EventOnTeamNoneUnit
  (|CallParentFunction)
  (Collision|SetCollisionResponsetoChannel (Variables|Default|GetTankBody) "ECC_GameTraceChannel1" "ECR_Ignore")
  (Rendering|Material|SetMaterial (Variables|Default|GetTankBody) 0 "/Game/Geometry/Meshes/CubeMaterial.CubeMaterial")
  (Collision|SetCollisionResponsetoChannel (Variables|Default|GetTankBody) "ECC_GameTraceChannel2" "ECR_Block"))

(fn ConstructionScript
  (|CallParentFunction))