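; BP_Collector is a collector unit that carries wood, stone and food and delivers them to the game's totals.
; AddResources adds an amount to the carried count for the given resource type.
; DepositResources adds each carried count to the matching BP_GameMode total, then zeroes it.
; MoveUnit writes the destination to the TargetLocationKey blackboard key, leaving the movement itself outside this graph.
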(event Custom|AddResources
  (params (ResourceType :type EResourceType%20Enum :default "WOOD") (ResourceAmount :type Integer))
  (switch Utilities|FlowControl|Switch|SwitchonEResourceType ResourceType
    (:WOOD
      (Variables|Default|SetCollectedWood (+ (Variables|Default|GetCollectedWood) ResourceAmount)))
    (:FOOD
      (Variables|Default|SetCollectedFood (+ ResourceAmount (Variables|Default|GetCollectedFood))))
    (:STONE
      (Variables|Default|SetCollectedStone (+ ResourceAmount (Variables|Default|GetCollectedStone))))))

(event Custom|DepositResources
  (bind _asbp_game_mode (Utilities|Casting|CastToBP_GameMode (Game|GetGameMode)))
  (Utilities|FlowControl|Sequence
    (:then_0
      (Variables|/Game/Blueprints/Core/BP_GameMode.BP_GameMode_C|SetWoodCollected _asbp_game_mode (+ (Variables|/Game/Blueprints/Core/BP_GameMode.BP_GameMode_C|GetWoodCollected _asbp_game_mode) (Variables|Default|GetCollectedWood)))
      (Variables|Default|SetCollectedWood 0))
    (:then_1
      (Variables|/Game/Blueprints/Core/BP_GameMode.BP_GameMode_C|SetStoneCollected _asbp_game_mode (+ (Variables|/Game/Blueprints/Core/BP_GameMode.BP_GameMode_C|GetStoneCollected _asbp_game_mode) (Variables|Default|GetCollectedStone)))
      (Variables|Default|SetCollectedStone 0))
    (:then_2
      (Variables|/Game/Blueprints/Core/BP_GameMode.BP_GameMode_C|SetFoodCollected _asbp_game_mode (+ (Variables|/Game/Blueprints/Core/BP_GameMode.BP_GameMode_C|GetFoodCollected _asbp_game_mode) (Variables|Default|GetCollectedFood)))
      (Variables|Default|SetCollectedFood 0))))

(event EventBeginPlay
  (|CallParentFunction))

(event Collision|EventActorBeginOverlap
  (params (OtherActor :type Actor%20Object%20Reference))
  (|CallParentFunction OtherActor) ; This node is disabled and will not be called.\nDrag off pins to build functionality.
)

(event EventTick
  (params (DeltaSeconds :type Float%20%28single-precision%29))
  (|CallParentFunction DeltaSeconds) ; This node is disabled and will not be called.\nDrag off pins to build functionality.
)

(event EventMoveUnit
  (params (Location :type Vector :default "0, 0, 0"))
  (AI|Components|Blackboard|SetValueasVector (AI|GetBlackboard 0) (Utilities|Name|MakeLiteralName "TargetLocationKey") Location))

(fn ConstructionScript
  (|CallParentFunction))