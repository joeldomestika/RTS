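; Camera pawn that implements mouse edge scrolling, moving its root component according to cursor position in the viewport.
; Each Tick runs horizontal and vertical checks that scale opposing X and Y offsets through NormalizeValue, a clamped range helper, using a percentage border.
; The far-edge ranges start beyond the viewport size, so their negative offsets apply at full strength across the screen.
; A separate MoveLeft event repeats the left-edge logic with BorderPercent and debug printing.
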(event Custom|Move%20Left
  (bind _returnvalue (Class|WidgetLayoutLibrary|GetMousePositiononViewport))
  (bind _asbp_game_mode (Utilities|Casting|CastToBP_GameMode (Game|GetGameMode)))
  (Transformation|AddRelativeLocation (Variables|Transformation|GetRootComponent) (* "10.000000, 0, 0" (- 1.0 (Math|Float|Clamp(Float) (Math|Float|NormalizetoRange (.x _returnvalue) 0.0 (* (.x (Viewport|GetViewportSize)) (/ (Variables|Default|GetBorderPercent) 1e+02)))))) false false)
  (Development|PrintString (Utilities|String|ToString(Vector) (* "10.000000, 0, 0" (- 1.0 (Math|Float|Clamp(Float) (Math|Float|NormalizetoRange (.x _returnvalue) 0.0 (* (.x (Viewport|GetViewportSize)) (/ (Variables|Default|GetBorderPercent) 1e+02)))))))))

(event Custom|Check%20Vertical%20Movement
  (params (Percentage :type Float%20%28single-precision%29))
  (bind _returnvalue (/ Percentage 1e+02))
  (bind _returnvalue_2 (Viewport|GetViewportSize))
  (bind _returnvalue_3 (* (.y _returnvalue_2) _returnvalue))
  (bind _returnvalue_4 (Class|WidgetLayoutLibrary|GetMousePositiononViewport))
  (Utilities|FlowControl|Sequence
    (:then_0
      (bind _normalizedvalue (CallFunction|NormalizeValue (.y _returnvalue_4) 0.0 _returnvalue_3))
      (Transformation|AddRelativeLocation (Variables|Transformation|GetRootComponent) (* "0.000000,10.000000, 0" (- 1.0 _normalizedvalue)) false false))
    (:then_1
      (bind _normalizedvalue_2 (CallFunction|NormalizeValue (.y _returnvalue_4) (+ _returnvalue_3 (.y (Viewport|GetViewportSize))) (.y (Viewport|GetViewportSize))))
      (Transformation|AddRelativeLocation (Variables|Transformation|GetRootComponent) (* "0.000000,-10.000000, 0" _normalizedvalue_2) false false))))

(event Custom|Check%20Horizontal%20Movement
  (params (Percentage :type Float%20%28single-precision%29))
  (bind _returnvalue (/ Percentage 1e+02))
  (bind _returnvalue_2 (Viewport|GetViewportSize))
  (bind _returnvalue_3 (* (.x _returnvalue_2) _returnvalue))
  (bind _returnvalue_4 (Class|WidgetLayoutLibrary|GetMousePositiononViewport))
  (Utilities|FlowControl|Sequence
    (:then_0
      (bind _normalizedvalue (CallFunction|NormalizeValue (.x _returnvalue_4) 0.0 _returnvalue_3))
      (Transformation|AddRelativeLocation (Variables|Transformation|GetRootComponent) (* "10.000000, 0, 0" (- 1.0 _normalizedvalue)) false false))
    (:then_1
      (bind _normalizedvalue_2 (CallFunction|NormalizeValue (.x _returnvalue_4) (+ _returnvalue_3 (.x (Viewport|GetViewportSize))) (.x (Viewport|GetViewportSize))))
      (Transformation|AddRelativeLocation (Variables|Transformation|GetRootComponent) (* "-10.000000, 0, 0" _normalizedvalue_2) false false))))

(event EventTick
  (params (DeltaSeconds :type Float%20%28single-precision%29))
  (CallFunction|CheckHorizontalMovement 3e+01)
  (CallFunction|CheckVerticalMovement 3e+01))

(fn ConstructionScript)

(fn NormalizeValue
  (params (Value :type Float%20%28single-precision%29) (Minimum :type Float%20%28single-precision%29) (Maximum :type Float%20%28single-precision%29))
  (return (Math|Float|Clamp(Float) (Math|Float|NormalizetoRange Value Minimum Maximum))))