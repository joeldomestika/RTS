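; BP_Opponent is the pawn or character for the AI opponent, acting as the entry point for registering that opponent's units.
; On BeginPlay it casts its controller to BP_AIControllerOpponent and caches the reference.
; Add and Remove events for tanks, assault vehicles and soldiers forward each unit to that controller after a validity check, so the unit logic itself lives in the controller.
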(event Custom|RemoveSoldier
  (params (Soldier :type BP%20Soldier%20Object%20Reference))
  (bind _aicontrolleropponent (Variables|Default|GetAIControllerOpponent)
    (:then
      (Default|RemoveSoldier _aicontrolleropponent Soldier))
    (:else)))

(event Custom|RemoveTank
  (params (Tank :type BP%20Tank%20Object%20Reference))
  (bind _aicontrolleropponent (Variables|Default|GetAIControllerOpponent)
    (:then
      (Default|RemoveTank _aicontrolleropponent Tank))
    (:else)))

(event Custom|RemoveAssaultVehicle
  (params (AssaultVehicle :type BP%20Assault%20Vehicle%20Object%20Reference))
  (bind _aicontrolleropponent (Variables|Default|GetAIControllerOpponent)
    (:then
      (Default|RemoveAssaultVehicle _aicontrolleropponent AssaultVehicle))
    (:else)))

(event Custom|AddTank
  (params (Tank :type BP%20Tank%20Object%20Reference))
  (bind _aicontrolleropponent (Variables|Default|GetAIControllerOpponent)
    (:then
      (Default|AddTank _aicontrolleropponent Tank))
    (:else)))

(event Custom|AddAssaultVehicle
  (params (AssaultVehicle :type BP%20Assault%20Vehicle%20Object%20Reference))
  (bind _aicontrolleropponent (Variables|Default|GetAIControllerOpponent)
    (:then
      (Default|AddAssaultVehicle _aicontrolleropponent AssaultVehicle))
    (:else)))

(event Custom|AddSoldier
  (params (Soldier :type BP%20Soldier%20Object%20Reference))
  (bind _aicontrolleropponent (Variables|Default|GetAIControllerOpponent)
    (:then
      (Default|AddSoldier _aicontrolleropponent Soldier))
    (:else)))

(event EventBeginPlay
  (bind _asbp_aicontroller_opponent (Utilities|Casting|CastToBP_AIControllerOpponent (AI|GetAIController 0)))
  (Variables|Default|SetAIControllerOpponent _asbp_aicontroller_opponent))

(event Collision|EventActorBeginOverlap
  (params (OtherActor :type Actor%20Object%20Reference)))

(event EventTick
  (params (DeltaSeconds :type Float%20%28single-precision%29)))

(fn ConstructionScript)